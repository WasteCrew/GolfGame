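; Golf ball pawn Blueprint that runs a timed button-mash challenge through its MashInput component.
; On BeginPlay it sets the component's input action, starts mashing with a target value and time limit, and prints a seconds-remaining countdown using a looping DoN and Delay.
; When mashing ends, it prints the final value and whether the player passed; no ball movement or other gameplay logic is present.
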(event `self.ReceiveBeginPlay`
  (bind _mashinput (`self.MashInput`))
  (`MashButtonInput.SetKeys` _mashinput "Mash1" true)
  (`MashButtonInput.StartMashing` _mashinput 15.0 5.0)
  (bind _counter (`/Engine/EditorBlueprintResources/StandardMacros.Do N` 6 :!label _label)
    (:`Exit`
      (if (!= _counter 6)
        (`KismetSystemLibrary.PrintString` (`KismetStringLibrary.Concat_StrStr` (`KismetStringLibrary.Conv_IntToString` (- 6 _counter)) " seconds remaining!"))
        (`KismetSystemLibrary.Delay` 1.0)
        (goto _label)))))

(event `self.MashInput.OnMashEnded`
  (params (bPassedEvent :type Boolean) (FinalMashValue :type "Float (single-precision)"))
  (`KismetSystemLibrary.PrintString` (`KismetStringLibrary.Concat_StrStr` "Final Value: " (`KismetStringLibrary.Conv_DoubleToString` FinalMashValue)))
  (`KismetSystemLibrary.PrintString` (select `bool` bPassedEvent :`false` "You failed!" :`true` "You passed!")))

(fn `UserConstructionScript`)